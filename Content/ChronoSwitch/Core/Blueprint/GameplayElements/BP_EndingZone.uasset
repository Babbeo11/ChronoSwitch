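; End-of-game trigger zone that starts the finale once two ChronoSwitch characters overlap its box.
; It disables collision, sets time switching to Personal and flags both players as Endgame.
; The authority runs randomly delayed timers that flip players between timelines using a vertical offset.
; StartCredits blocks movement input, swaps soundscapes for the ending theme, then after a delay silences both Balls, shows the credits widget and clears the timer.
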(event OnComponentBeginOverlap(Box)
  (params (OverlappedComponent :type Primitive%20Component%20Object%20Reference) (OtherActor :type Actor%20Object%20Reference) (OtherComp :type Primitive%20Component%20Object%20Reference) (OtherBodyIndex :type Integer) (bFromSweep :type Boolean) (SweepResult :type Hit%20Result%20Structure%20%28by%20ref%29))
  (bind _returnvalue (Class|ChronoSwitchBlueprintLibrary|GetChronoGameState))
  (bind _as_bp_chrono_switch_character (Variables|Default|GetAs%20BP%20Chrono%20Switch%20Character))
  (bind _asbp_chrono_switch_character (Utilities|Casting|CastToBP_ChronoSwitchCharacter OtherActor))
  (Utilities|Array|AddUnique _as_bp_chrono_switch_character _asbp_chrono_switch_character)
  (if (== (Utilities|Array|Length _as_bp_chrono_switch_character) 2)
    (Utilities|FlowControl|DoOnce false
      (:Completed
        (Collision|SetCollisionEnabled (Variables|Default|GetBox) "NoCollision")
        (Utilities|IsValid _returnvalue
          (:Is%20Valid
            (Class|ChronoSwitchGameState|SetTimeSwitchMode _returnvalue "Personal")
            (for _array_element (Variables|Default|GetAs%20BP%20Chrono%20Switch%20Character)
              (Variables|/Script/ChronoSwitch.ChronoSwitchCharacter|SetEndgame _array_element true))
            (Networking|SwitchHasAuthority
              (:Authority
                (CallFunction|StartCredits)
                (Utilities|Time|SetTimerbyEvent (EventDispatchers|CreateEvent :!event Custom|TeleportPlayers) 0.1 false false 2.0))
              (:Remote
                (CallFunction|StartCredits)))))))))

(event OnComponentEndOverlap(Box)
  (params (OverlappedComponent :type Primitive%20Component%20Object%20Reference) (OtherActor :type Actor%20Object%20Reference) (OtherComp :type Primitive%20Component%20Object%20Reference) (OtherBodyIndex :type Integer))
  (Utilities|Casting|CastToBP_ChronoSwitchCharacter OtherActor)
  (Utilities|Array|RemoveItem (Variables|Default|GetAs%20BP%20Chrono%20Switch%20Character) 0))

(event Custom|StartCredits
  (bind _returnvalue (Game|GetPlayerController 0))
  (bind _ball2 (Variables|Default|Getball2))
  (bind _ball (Variables|Default|Getball))
  (Utilities|FlowControl|DoOnce false
    (:Completed
      (Input|SetIgnoreMoveInput _returnvalue true)
      (bind _asbp_chrono_switch_character (Utilities|Casting|CastToBP_ChronoSwitchCharacter (Pawn|GetControlledPawn _returnvalue)))
      (Audio|Components|Audio|AdjustVolume (Variables|/Game/ChronoSwitch/Core/Characters/BP_ChronoSwitchCharacter.BP_ChronoSwitchCharacter_C|GetMS_SoundscapeFuture _asbp_chrono_switch_character) 0.0 0.0 "Linear" :!class /Script/Engine.AudioComponent)
      (Audio|Components|Audio|AdjustVolume (Variables|/Game/ChronoSwitch/Core/Characters/BP_ChronoSwitchCharacter.BP_ChronoSwitchCharacter_C|GetMS_Soundscape _asbp_chrono_switch_character) 0.0 0.0 "Linear" :!class /Script/Engine.AudioComponent)
      (Audio|PlaySound2D "/Game/ChronoSwitch/Sound/Chronoswitch_ending_theme.Chronoswitch_ending_theme" 1.0 1.0 0.0 0 0)
      (Utilities|IsValid _ball
        (:Is%20Valid
          (Utilities|IsValid _ball2
            (:Is%20Valid
              (Utilities|FlowControl|Delay 12.0)
              (Audio|Components|Audio|Stop (Variables|/Script/Engine.AmbientSound|GetAudioComponent _ball))
              (Audio|Components|Audio|Stop (Variables|/Script/Engine.AmbientSound|GetAudioComponent _ball2))
              (bind _returnvalue_2 (UserInterface|CreateWidget "/Game/ChronoSwitch/Core/UI/WBP_Credits.WBP_Credits_C" _returnvalue))
              (UserInterface|Viewport|AddtoViewport _returnvalue_2 0)
              (Utilities|Time|ClearandInvalidateTimerbyHandle (Variables|Default|GetTimerRef)))))))))

(event Custom|TeleportPlayers
  (for _array_element (Variables|Default|GetAs%20BP%20Chrono%20Switch%20Character)
    (Utilities|IsValid _array_element
      (:Is%20Valid
        (if (> (.z (Transformation|GetActorLocation _array_element)) -2e+03)
          (Default|ClientExecuteTimeSwitchLogic _array_element false "0, 0, 0")
          (Transformation|SetActorLocation _array_element (Math|Vector|MakeVector (.x (Transformation|GetActorLocation _array_element)) (.y (Transformation|GetActorLocation _array_element)) (- (.z (Transformation|GetActorLocation _array_element)) 4485.0)) false true)
          (else
            (Default|ClientExecuteTimeSwitchLogic _array_element true (Math|Vector|MakeVector (.x (Transformation|GetActorLocation _array_element)) (.y (Transformation|GetActorLocation _array_element)) (+ (.z (Transformation|GetActorLocation _array_element)) 4485.0))))))))
  (bind _returnvalue (Utilities|Time|SetTimerbyEvent (EventDispatchers|CreateEvent :!event Custom|TeleportPlayers) 0.1 false false (Math|Random|RandomFloatinRange 0.8 1.5)))
  (Variables|Default|SetTimerRef _returnvalue))

(fn ConstructionScript)