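; Player controller for ChronoSwitch that toggles a Future flag on the E key to test time-swap materials.
; Each press sets flash color and curve parameters in the MC_TimeSwap material parameter collection.
; One timeline plays when leaving Future and reverses when entering it, writing its TimeSwap track to the Material State parameter to animate the transition.
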(event EventBeginPlay)

(event EventTick
  (params (DeltaSeconds :type Float%20%28single-precision%29)))

(event Input|KeyboardEvents|E
  (params (Key :type Key%20Structure :default "None"))
  (bind _parameter_value (Variables|Default|GetParameter%20Value))
  ;[0.009677 0.15 0 0.5] Material Testing
  (:Pressed
    (if (Variables|Default|GetFuture)
      (Variables|Default|SetFuture false)
      (Rendering|Material|SetVectorParameterValue "/Game/ChronoSwitch/Materials/Collections/MC_TimeSwap.MC_TimeSwap" "FlashColor" (Utilities|Array|Get(acopy) _parameter_value) :!class /Script/Engine.KismetMaterialLibrary)
      (Rendering|Material|SetScalarParameterValue "/Game/ChronoSwitch/Materials/Collections/MC_TimeSwap.MC_TimeSwap" "FlashCurve" 0.0 :!class /Script/Engine.KismetMaterialLibrary)
      (bind _timeswap (Timeline|Timeline Play)
        (:Update
          (Rendering|Material|SetScalarParameterValue "/Game/ChronoSwitch/Materials/Collections/MC_TimeSwap.MC_TimeSwap" "Material State" _timeswap :!class /Script/Engine.KismetMaterialLibrary)))
      (else
        (Variables|Default|SetFuture true)
        (Rendering|Material|SetVectorParameterValue "/Game/ChronoSwitch/Materials/Collections/MC_TimeSwap.MC_TimeSwap" "FlashColor" (Utilities|Array|Get(acopy) _parameter_value 1) :!class /Script/Engine.KismetMaterialLibrary)
        (Rendering|Material|SetScalarParameterValue "/Game/ChronoSwitch/Materials/Collections/MC_TimeSwap.MC_TimeSwap" "FlashCurve" 1.0 :!class /Script/Engine.KismetMaterialLibrary)
        (Timeline|Timeline Reverse)))))

(fn ConstructionScript)