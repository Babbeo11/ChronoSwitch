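; Blockout door that opens by sliding its static mesh vertically, with replicated open state.
; OpenDoor sets IsDoorOpen and calls DoorAnimation, which plays a timeline that maps its track to the mesh's relative Z, up to 240 units.
; The IsDoorOpen RepNotify also triggers the animation, so the movement follows the replicated state.
; The file contains no closing logic.
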(event Custom|OpenDoor
  (Variables|Default|SetIsDoorOpen true)
  (CallFunction|DoorAnimation))

(event Custom|DoorAnimation
  (bind _staticmesh (Variables|Default|GetStaticMesh))
  (bind _relativelocation (Variables|/Script/Engine.SceneComponent|GetRelativeLocation _staticmesh))
  (bind _newtrack_0 (Timeline|Timeline Play)
    (:Update
      (Transformation|SetRelativeLocation _staticmesh (Math|Vector|MakeVector (.x _relativelocation) (.y _relativelocation) (Math|Float|MapRangeClamped _newtrack_0 0.0 1.0 0.0 2.4e+02)) false false))))

(event EventBeginPlay)

(event Collision|EventActorBeginOverlap
  (params (OtherActor :type Actor%20Object%20Reference)))

(event EventTick
  (params (DeltaSeconds :type Float%20%28single-precision%29)))

(fn ConstructionScript)

(fn OnRepIsDoorOpen
  (Variables|Default|GetIsDoorOpen
    (:then
      (CallFunction|DoorAnimation))
    (:else)))