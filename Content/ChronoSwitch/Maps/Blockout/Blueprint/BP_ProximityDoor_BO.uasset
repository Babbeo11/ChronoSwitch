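; Blockout two-panel sliding door that opens when at least two ChronoSwitch characters stand in its Box trigger.
; Overlap counts drive a timeline that slides both meshes along local Y, reversing when the count drops below two.
; A second trigger, Box1, sets IsBlocked once two characters are inside, latching the door against reopening.
; Both counters have RepNotify handlers that refresh the door or blocked state.
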(event OnComponentBeginOverlap(Box)
  (params (OverlappedComponent :type Primitive%20Component%20Object%20Reference) (OtherActor :type Actor%20Object%20Reference) (OtherComp :type Primitive%20Component%20Object%20Reference) (OtherBodyIndex :type Integer) (bFromSweep :type Boolean) (SweepResult :type Hit%20Result%20Structure%20%28by%20ref%29))
  (Utilities|Casting|CastToBP_ChronoSwitchCharacter OtherActor)
  (Math|Integer|IncrementInt (Variables|Default|GetIndex)
    (:%20%20
      (CallFunction|UpdateDoorVisual))))

(event OnComponentEndOverlap(Box)
  (params (OverlappedComponent :type Primitive%20Component%20Object%20Reference) (OtherActor :type Actor%20Object%20Reference) (OtherComp :type Primitive%20Component%20Object%20Reference) (OtherBodyIndex :type Integer))
  (Utilities|Casting|CastToBP_ChronoSwitchCharacter OtherActor)
  (Math|Integer|DecrementInt (Variables|Default|GetIndex)
    (:%20%20
      (CallFunction|UpdateDoorVisual))))

(event OnComponentBeginOverlap(Box1)
  (params (OverlappedComponent :type Primitive%20Component%20Object%20Reference) (OtherActor :type Actor%20Object%20Reference) (OtherComp :type Primitive%20Component%20Object%20Reference) (OtherBodyIndex :type Integer) (bFromSweep :type Boolean) (SweepResult :type Hit%20Result%20Structure%20%28by%20ref%29))
  (Utilities|Casting|CastToBP_ChronoSwitchCharacter OtherActor)
  (Math|Integer|IncrementInt (Variables|Default|GetIndex2)
    (:%20%20
      (if (>= (Variables|Default|GetIndex2) 2)
        (Variables|Default|SetIsBlocked true)))))

(event OnComponentEndOverlap(Box1)
  (params (OverlappedComponent :type Primitive%20Component%20Object%20Reference) (OtherActor :type Actor%20Object%20Reference) (OtherComp :type Primitive%20Component%20Object%20Reference) (OtherBodyIndex :type Integer))
  (Utilities|Casting|CastToBP_ChronoSwitchCharacter OtherActor)
  (Variables|Default|GetIsBlocked
    (:then)
    (:else
      (Math|Integer|DecrementInt (Variables|Default|GetIndex2)))))

(event Custom|UpdateDoorVisual
  (bind _staticmesh (Variables|Default|GetStaticMesh))
  (bind _staticmesh1 (Variables|Default|GetStaticMesh1))
  (bind _relativelocation (Variables|/Script/Engine.SceneComponent|GetRelativeLocation _staticmesh))
  (bind _relativelocation_2 (Variables|/Script/Engine.SceneComponent|GetRelativeLocation _staticmesh1))
  (if (>= (Variables|Default|GetIndex) 2)
    (Variables|Default|GetIsBlocked
      (:then)
      (:else
        (bind _newtrack_0 (Timeline|DoorAnimation Play)
          (:Update
            (Transformation|SetRelativeLocation (Variables|Default|GetStaticMesh1) (Math|Vector|MakeVector (.x _relativelocation_2) (Math|Float|MapRangeClamped _newtrack_0 0.0 1.0 0.0 1e+02) (.z _relativelocation_2)) false false)
            (Transformation|SetRelativeLocation (Variables|Default|GetStaticMesh) (Math|Vector|MakeVector (.x _relativelocation) (Math|Float|MapRangeClamped _newtrack_0 0.0 1.0 -4e+02 -5e+02) (.z _relativelocation)) false false)))))
    (else
      (Timeline|DoorAnimation Reverse))))

(event EventBeginPlay)

(event Collision|EventActorBeginOverlap
  (params (OtherActor :type Actor%20Object%20Reference)))

(event EventTick
  (params (DeltaSeconds :type Float%20%28single-precision%29)))

(fn ConstructionScript)

(fn OnRepIndex
  (CallFunction|UpdateDoorVisual))

(fn OnRepIndex2
  (if (>= (Variables|Default|GetIndex2) 2)
    (Variables|Default|SetIsBlocked true)))