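; Spline-driven wire prop that rebuilds in the Construction Script from one of six selectable wire variants.
; SplineMeshVar chooses segment layout: one spline mesh per point pair, or evenly spaced segments by distance with scaled direction tangents.
; Each segment gets uniform scaling and dynamic MI_Wire instances driven by exposed color, dirt, specular, roughness and texture choices.
; Variants 3 to 5 take a second material slot with its own color.
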(fn ConstructionScript
  (|Wire))